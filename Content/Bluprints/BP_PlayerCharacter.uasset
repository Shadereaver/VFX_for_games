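; Player character Blueprint that triggers ring and lightning effects, apparently Niagara, in response to a hit event.
; When the ring is inactive, a hit toggles both effects and starts two timers.
; A fast looping timer feeds the actor's location and capsule forward vector into the ring's position variables.
; A three-second timer stops that feed and toggles the lightning again, leaving the ring untouched.
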(event Custom|Effect%20done
  (Utilities|Time|ClearandInvalidateTimerbyHandle (Variables|Default|GetPassRingDataHandle))
  (Components|Activation|ToggleActive (Variables|Default|GetNS_Lightning)))

(event Custom|Pass%20ring%20data
  (Class|NiagaraComponent|SetVariablePosition (Variables|Default|GetNS_Ring) "PlayerPos" (Transformation|GetActorLocation))
  (Class|NiagaraComponent|SetVariablePosition (Variables|Default|GetNS_Ring) "RingFacing" (Math|Vector|GetForwardVector (Variables|Default|GetCapsuleComponent))))

(event Custom|Handle_OnHit_1
  (params (HitComponent :type Primitive%20Component%20Object%20Reference) (OtherActor :type Actor%20Object%20Reference) (OtherComp :type Primitive%20Component%20Object%20Reference) (NormalImpulse :type Vector) (Hit :type Hit%20Result%20Structure%20%28by%20ref%29))
  (bind _ns_ring (Variables|Default|GetNS_Ring))
  (if (not (Components|Activation|IsActive _ns_ring))
    (Components|Activation|ToggleActive _ns_ring)
    (Utilities|Time|SetTimerbyEvent (delegate Custom|Effect%20done) 3.0)
    (bind _returnvalue (Utilities|Time|SetTimerbyEvent (delegate Custom|Pass%20ring%20data) 0.01 true))
    (Variables|Default|SetPassRingDataHandle _returnvalue)))

(fn ConstructionScript)