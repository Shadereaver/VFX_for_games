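; BP_Enemy is an enemy Blueprint that can swap positions with another actor through its StartSwap event.
; The SwapTimelie graph captures both starting locations, then plays the Swap timeline to lerp each actor toward the other's spot.
; The timeline's vector track offsets the two actors in opposite directions during the move.
; When the timeline finishes, SwapDone is called.
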(event EventStartSwap
  (params (OtherActor :type Actor%20Object%20Reference))
  (Variables|Ability3|SetOther%20Actor OtherActor)
  (|SwapTimelie
    (:Finished
      (Class|PlayerCharacter|SwapDone))))

(fn ConstructionScript)